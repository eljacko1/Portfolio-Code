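; TutorialBlueprint runs a minutes-and-seconds countdown that ends in a game over screen.
; While TimerActive is set, Tick passes through a one-second Delay to decrement TimeSec, rolling over into TimeMin, instead of using a timer.
; When the minutes drop below zero, it clears all widgets, shows GameOver_Widget and switches the player to UI-only input with a visible cursor.
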(event `self.ReceiveTick`
  (params (DeltaSeconds :type "Float (single-precision)"))
  (bind _returnvalue (`GameplayStatics.GetPlayerController` 0))
  (if (`self.TimerActive`)
    (`KismetSystemLibrary.Delay` 1.0)
    (set `self.TimeSec` (- (`self.TimeSec`) 1))
    (if (< (`self.TimeSec`) 0)
      (set `self.TimeMin` (- (`self.TimeMin`) 1))
      (set `self.TimeSec` 59)
      (if (< (`self.TimeMin`) 0)
        (`WidgetLayoutLibrary.RemoveAllWidgets`)
        (bind _returnvalue_2 (`|CreateWidget` "/Game/UI/GameOver_Widget.GameOver_Widget_C"))
        (`UserWidget.AddToViewport` _returnvalue_2 0)
        (set `PlayerController.bShowMouseCursor` true _returnvalue)
        (`WidgetBlueprintLibrary.SetInputMode_UIOnlyEx` _returnvalue _returnvalue_2)))))

(fn `UserConstructionScript`)
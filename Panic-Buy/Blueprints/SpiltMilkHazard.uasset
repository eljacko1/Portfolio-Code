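; SpiltMilkHazard is a spilt milk hazard actor that appears intended to spin the player after a slip.
; Any overlap with its Box sets Slipping, which makes Tick apply a local rotation to Player_BP every frame.
; That rotation is currently zero because the RotationSpeed yaw calculation is disconnected.
; The one-second delay that clears Slipping never runs, so the flag stays set once triggered.
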(event `self.ReceiveTick`
  (params (DeltaSeconds :type "Float (single-precision)"))
  (if (`self.Slipping`)
    (bind _asplayer_bp (cast `/Game/Blueprints/Player_BP` (`GameplayStatics.GetPlayerCharacter` 0)))
    (`self.K2_AddActorLocalRotation` :`self` _asplayer_bp)))

(event `self.Box.OnComponentBeginOverlap`
  (params (OverlappedComponent :type "PrimitiveComponent Object Reference") (OtherActor :type "Actor Object Reference") (OtherComp :type "PrimitiveComponent Object Reference") (OtherBodyIndex :type Integer) (bFromSweep :type Boolean) (SweepResult :type "HitResult Structure (by ref)"))
  (set `self.Slipping` true))

(fn `UserConstructionScript`)
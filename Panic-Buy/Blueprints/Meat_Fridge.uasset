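; Meat fridge actor with two hinged doors that the player opens and closes with E.
; Per-door collision volumes enable interaction when the player overlaps, with the left door taking priority.
; Timelines drive each pivot's world yaw, playing forward or in reverse, while the actor's input is disabled during the swing.
; Ending overlap disables that door, first auto-closing it through a separate timeline if left open.
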(event `self.ReceiveBeginPlay`
  (`self.EnableInput` (`GameplayStatics.GetPlayerController` 0)))

(event `self.Door_CollisionL.OnComponentBeginOverlap`
  (params (OverlappedComponent :type "PrimitiveComponent Object Reference") (OtherActor :type "Actor Object Reference") (OtherComp :type "PrimitiveComponent Object Reference") (OtherBodyIndex :type Integer) (bFromSweep :type Boolean) (SweepResult :type "HitResult Structure (by ref)"))
  ;[1 1 1] Enable / Disable Input LDoor
  (bind _asplayer_bp (cast `/Game/Blueprints/Player_BP` (`GameplayStatics.GetPlayerCharacter` 0)))
  (if (== OtherActor _asplayer_bp)
    (set `self.DoorLEnabled` true)))

(event `self.Door_CollisionR.OnComponentBeginOverlap`
  (params (OverlappedComponent :type "PrimitiveComponent Object Reference") (OtherActor :type "Actor Object Reference") (OtherComp :type "PrimitiveComponent Object Reference") (OtherBodyIndex :type Integer) (bFromSweep :type Boolean) (SweepResult :type "HitResult Structure (by ref)"))
  ;[1 1 1] Enable/Disable Input RDoor
  (bind _asplayer_bp (cast `/Game/Blueprints/Player_BP` (`GameplayStatics.GetPlayerCharacter` 0)))
  (if (== OtherActor _asplayer_bp)
    (set `self.DoorREnabled` true)))

(event `self.Door_CollisionL.OnComponentEndOverlap`
  (params (OverlappedComponent :type "PrimitiveComponent Object Reference") (OtherActor :type "Actor Object Reference") (OtherComp :type "PrimitiveComponent Object Reference") (OtherBodyIndex :type Integer))
  ;[1 1 1] Enable / Disable Input LDoor
  (if (`self.Door Closed L`)
    (set `self.DoorLEnabled` false)
    (else
      (bind (_direction _newtrack_0) (`Timeline|Timeline_1` :!via `ReverseFromEnd`)
        (:`Update`
          (`SceneComponent.K2_SetWorldRotation` (`self.PivotL`) (`KismetMathLibrary.MakeRotator` 0.0 0.0 _newtrack_0) false false))
        (:`Finished`
          (set `self.DoorLEnabled` false)
          (set `self.Door Closed L` true))))))

(event `self.Door_CollisionR.OnComponentEndOverlap`
  (params (OverlappedComponent :type "PrimitiveComponent Object Reference") (OtherActor :type "Actor Object Reference") (OtherComp :type "PrimitiveComponent Object Reference") (OtherBodyIndex :type Integer))
  ;[1 1 1] Enable/Disable Input RDoor
  (if (`self.Door Closed R`)
    (set `self.DoorREnabled` false)
    (else
      (bind (_direction _newtrack_0) (`Timeline|Timeline_0` :!via `ReverseFromEnd`)
        (:`Update`
          (`SceneComponent.K2_SetWorldRotation` (`self.PivotR`) (`KismetMathLibrary.MakeRotator` 0.0 0.0 _newtrack_0) false false))
        (:`Finished`
          (set `self.DoorREnabled` false)
          (set `self.Door Closed R` true))))))

(event `Key|E`
  (params (Key :type "Key Structure"))
  (bind _returnvalue (`GameplayStatics.GetPlayerController` 0))
  (:`Pressed`
    (if (`self.DoorLEnabled`)
      (`self.DisableInput` _returnvalue)
      ;[1 1 1] Open/Close door L
      (if (`self.Door Closed L`)
        (set `self.Door Closed L` false)
        (bind (_direction _newtrack_0) (`Timeline|Open/Close door L` :!via `PlayFromStart` :!label _label)
          (:`Update`
            (`SceneComponent.K2_SetWorldRotation` (`self.PivotL`) (`KismetMathLibrary.MakeRotator` 0.0 0.0 _newtrack_0) false false))
          (:`Finished`
            (`self.EnableInput` (`GameplayStatics.GetPlayerController` 0))))
        (else
          (set `self.Door Closed L` true)
          (goto _label :!via `ReverseFromEnd`)))
      (else
        (`self.DisableInput` _returnvalue)
        (if (`self.DoorREnabled`)
          ;[1 1 1] Open/Close door R
          (if (`self.Door Closed R`)
            (set `self.Door Closed R` false)
            (bind (_direction_2 _newtrack_0_2) (`Timeline|Open/Close door R` :!via `PlayFromStart` :!label _label_2)
              (:`Update`
                (`SceneComponent.K2_SetWorldRotation` (`self.PivotR`) (`KismetMathLibrary.MakeRotator` 0.0 0.0 _newtrack_0_2) false false))
              (:`Finished`
                (`self.EnableInput` (`GameplayStatics.GetPlayerController` 0))))
            (else
              (set `self.Door Closed R` true)
              (goto _label_2 :!via `ReverseFromEnd`))))))))

(fn `UserConstructionScript`)
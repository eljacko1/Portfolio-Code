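; Payment card actor for a card-swipe minigame that ends the current level once a swipe is accepted.
; While its mesh is visible, Interact disables input and plays a timeline swiping the card along a fixed offset.
; A swipe passes on a random target attempt or a random speed roll; otherwise Player_BP's CardMessage says swipe slower or faster and input returns.
; Acceptance reverses the card while streaming in MainMenu and unloading the current level.
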(event `self.ReceiveBeginPlay`
  (set `self.Start Location` (`self.K2_GetActorLocation`))
  (set `self.NumberofSwipes` (`KismetMathLibrary.RandomIntegerInRange` 0 7)))

(event `InputAction|Interact` :consume false
  (params (Key :type "Key Structure"))
  (bind _returnvalue (`GameplayStatics.GetPlayerCharacter` 0))
  (bind _start_location (`self.Start Location`))
  (bind _start_location_2 (`self.Start Location`))
  (bind _start_location_3 (`self.Start Location`))
  (bind _start_location_4 (`self.Start Location`))
  (:`Pressed`
    (if (`SceneComponent.bVisible` (`self.StaticMeshComponent`))
      (`self.DisableInput` (`GameplayStatics.GetPlayerController` 0))
      (set `self.CurrentSwipe` (+ (`self.CurrentSwipe`) 1))
      (bind (_direction _newtrack_4) (`Timeline|Timeline_0` :!via `PlayFromStart`)
        (:`Update`
          (`self.K2_SetActorLocation` (`KismetMathLibrary.VLerp` _start_location (+ _start_location (-31.0 10.0 -14.0)) _newtrack_4)))
        (:`Finished`
          (if (== (`self.CurrentSwipe`) (`self.NumberofSwipes`))
            (bind _asplayer_bp (cast `/Game/Blueprints/Player_BP` (`GameplayStatics.GetPlayerCharacter` 0) :!label _label))
            (set `/Game/Blueprints/Player_BP.CardMessage` "Card Accepted!" _asplayer_bp)
            (`self.DisableInput` (`GameplayStatics.GetPlayerController` 0))
            (`KismetSystemLibrary.Delay` 1.0)
            (bind (_direction_2 _newtrack_4_2) (`Timeline|Timeline_1` :!via `ReverseFromEnd`)
              (:`Update`
                (`self.K2_SetActorLocation` (`KismetMathLibrary.VLerp` _start_location_3 (+ _start_location_3 (-31.0 10.0 -14.0)) _newtrack_4_2))
                (bind _asmy_game_instance (cast `/Game/MyGameInstance` (`GameplayStatics.GetGameInstance`)))
                (`GameplayStatics.LoadStreamLevel` "MainMenu" true)
                (`GameplayStatics.UnloadStreamLevel` (`/Game/MyGameInstance.CurrentLevelName` _asmy_game_instance))))
            (else
              (bind _output_get (set `self.Speed` (`KismetMathLibrary.RandomIntegerInRange` 1 3)))
              (if (== _output_get 2)
                (goto _label)
                (elif (== (`self.Speed`) 1)
                  (bind _asplayer_bp_2 (cast `/Game/Blueprints/Player_BP` _returnvalue))
                  (set `/Game/Blueprints/Player_BP.CardMessage` "Card Declined: Swipe Slower!" _asplayer_bp_2)
                  (`KismetSystemLibrary.Delay` 1.0)
                  (bind (_direction_3 _newtrack_4_3) (`Timeline|Timeline_2` :!via `ReverseFromEnd`)
                    (:`Update`
                      (`self.K2_SetActorLocation` (`KismetMathLibrary.VLerp` _start_location_4 (+ _start_location_4 (-31.0 10.0 -14.0)) _newtrack_4_3)))
                    (:`Finished`
                      (`KismetSystemLibrary.Delay` 0.5 :!label _label_2)
                      (`self.EnableInput` (`GameplayStatics.GetPlayerController` 0))
                      (bind _asplayer_bp_3 (cast `/Game/Blueprints/Player_BP` (`GameplayStatics.GetPlayerCharacter` 0)))
                      (set `/Game/Blueprints/Player_BP.CardMessage` "" _asplayer_bp_3)))
                  (else
                    (bind _asplayer_bp_4 (cast `/Game/Blueprints/Player_BP` _returnvalue))
                    (set `/Game/Blueprints/Player_BP.CardMessage` "Card Declined: Swipe Faster!" _asplayer_bp_4)
                    (`KismetSystemLibrary.Delay` 1.0)
                    (bind (_direction_4 _newtrack_4_4) (`Timeline|Timeline_3` :!via `ReverseFromEnd`)
                      (:`Update`
                        (`self.K2_SetActorLocation` (`KismetMathLibrary.VLerp` _start_location_2 (+ _start_location_2 (-31.0 10.0 -14.0)) _newtrack_4_4)))
                      (:`Finished`
                        (goto _label_2)))))))))))))

(fn `UserConstructionScript`)